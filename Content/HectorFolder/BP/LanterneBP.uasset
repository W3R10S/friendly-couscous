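; LanterneBP is a lantern Blueprint that holds a Money value and marks itself dead when that value drops below zero.
; BeginPlay stores a self reference in MoneyReferance, resets Money to zero and prints it.
; GainMoney adds the given amount and prints the total, while Tick checks every frame for a negative balance to set IsDead.
; The RestoreBaseSpeed, GainSpeed and LoseSpeed functions are empty stubs.
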(event EventBeginPlay
  (Variables|Default|SetMoneyReferance self)
  (bind _output_get (Variables|Default|SetMoney 0.0))
  (Development|PrintString (Utilities|String|ToString(Float) _output_get)))

(event EventTick
  (params (DeltaSeconds :type Float%20%28single-precision%29))
  (if (< (Variables|Default|GetMoney) 0.0)
    (Variables|Default|SetIsDead true)))

(fn GainMoney
  (params (MoneyGain :type Float%20%28single-precision%29))
  (bind _output_get (Variables|Default|SetMoney (+ MoneyGain (Variables|Default|GetMoney))))
  (Development|PrintString (Utilities|String|ToString(Float) _output_get)))

(fn RestoreBaseSpeed)

(fn GainSpeed)

(fn LoseSpeed)