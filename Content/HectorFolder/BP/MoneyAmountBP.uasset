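; Actor component that tracks the money held by its owning FirstPersonCharacter and can slow that character as the money adds weight.
; BeginPlay resets Money, caches the character and records its base speed.
; GainMoney adds to the total.
; Each WeightManager call subtracts WeightAmount from walk speed while Money meets a threshold and max speed is above a floor, with debug prints throughout.
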(event EventBeginPlay
  (bind _output_get (Variables|Default|SetMoney 0.0))
  (Development|PrintString (Utilities|String|ToString(Float) _output_get))
  (bind _asfirst_person_character (Utilities|Casting|CastToFirstPersonCharacter (Components|GetOwner)))
  (Variables|Default|SetCharacter _asfirst_person_character)
  (Variables|Default|SetBaseSpeed (Class|MovementComponent|GetMaxSpeed (Variables|/Script/Engine.Character|GetCharacterMovement (Variables|Default|GetCharacter)))))

(event EventTick
  (params (DeltaSeconds :type Float%20%28single-precision%29)))

(fn GainMoney
  (params (MoneyGain :type Float%20%28single-precision%29))
  (bind _output_get (Variables|Default|SetMoney (+ MoneyGain (Variables|Default|GetMoney))))
  (Development|PrintString (Utilities|String|ToString(Float) _output_get)))

(fn WeightManager
  (bind _character (Variables|Default|GetCharacter))
  (bind _charactermovement (Variables|/Script/Engine.Character|GetCharacterMovement _character))
  (bind _returnvalue (Class|MovementComponent|GetMaxSpeed _charactermovement))
  (if (>= (Variables|Default|GetMoney) 11.0)
    (if (>= _returnvalue 1.5e+02)
      (bind _output_get (Variables|/Script/Engine.CharacterMovementComponent|SetMaxWalkSpeed _charactermovement (- _returnvalue (Variables|Default|GetWeightAmount))))
      (Development|PrintString (Utilities|String|ToString(Float) _output_get)))))