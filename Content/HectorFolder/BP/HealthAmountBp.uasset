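; HealthAmountBp is a health tracker Blueprint that starts Health at MaxHealth on BeginPlay.
; GainLife adds one point while Health is below MaxHealth.
; LoseLife subtracts HealthLost unless already dead, then sets IsDead once Health reaches zero or below.
; Each change prints the current Health as debug output, and Tick is unused.
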(event EventBeginPlay
  (bind _output_get (Variables|Default|SetHealth (Variables|Default|GetMaxHealth)))
  (Development|PrintString (Utilities|String|ToString(Float) _output_get)))

(event EventTick
  (params (DeltaSeconds :type Float%20%28single-precision%29)))

(fn GainLife
  (if (< (Variables|Default|GetHealth) (Variables|Default|GetMaxHealth))
    (bind _output_get (Variables|Default|SetHealth (+ 1.0 (Variables|Default|GetHealth))))
    (Development|PrintString (Utilities|String|ToString(Float) _output_get))))

(fn LoseLife
  (if (not (Variables|Default|GetIsDead))
    (bind _output_get (Variables|Default|SetHealth (- (Variables|Default|GetHealth) (Variables|Default|GetHealthLost))))
    (Development|PrintString (Utilities|String|ToString(Float) _output_get))
    (if (<= (Variables|Default|GetHealth) 0.0)
      (Variables|Default|SetIsDead true)
      (else
        (Variables|Default|SetIsDead false)))))